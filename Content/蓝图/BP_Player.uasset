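; BP_Player is a VR player Blueprint that gives the player a right hand wielding a lightsaber.
; The construction script calls 初始化左右手, which adds a BP_手 child actor mirrored on Y and attaches it to the right controller.
; BeginPlay sets the spectator screen to undistorted and activates that hand's lightsaber.
; Left-hand setup and lightsaber deactivation are present but never run.
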(event EventBeginPlay
  (Class|HeadMountedDisplayFunctionLibrary|SetSpectatorScreenMode "Undistorted")
  (Default|激活光剑 (Variables|Default|Get右手)))

(event Input|TouchEvents|OculusTouchRightTriggerClick
  (params (Key :type Key%20Structure :default "None")))

(event Input|KeyboardEvents|MotionControllerLeftGrip1
  (params (Key :type Key%20Structure :default "None")))

(fn ConstructionScript
  (|初始化左右手))