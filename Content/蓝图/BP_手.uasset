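; Hand actor with a lightsaber that extends, retracts and damages bp_方块 blocks it sweeps through.
; A timeline scales the blade on Z, enabling Tick shortly after extension and disabling it once retracted.
; Each Tick derives swing velocity and box-traces from the last blade position, oriented to blade and motion, avoiding reliance on overlaps.
; Hit blocks receive a damage message with velocity, swing-plane normal (cross product) and impact data.
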(event OnComponentBeginOverlap(剑)
  (params (OverlappedComponent :type Primitive%20Component%20Object%20Reference) (OtherActor :type Actor%20Object%20Reference) (OtherComp :type Primitive%20Component%20Object%20Reference) (OtherBodyIndex :type Integer) (bFromSweep :type Boolean) (SweepResult :type Hit%20Result%20Structure%20%28by%20ref%29)))

(event Custom|激活光剑
  (bind (_direction _新建轨迹_0) (Timeline|光剑动画 Play)
    (:Update
      (Transformation|SetRelativeScale3D (Variables|Default|GetScene1) (Math|Vector|MakeVector 1.0 1.0 _新建轨迹_0)))
    (:Finished
      (if (Utilities|Enum|Equal(Enum) _direction "Forward")
        (Variables|Default|Set上一帧位置 (Transformation|GetWorldLocation (Variables|Default|Get剑)))
        (Utilities|FlowControl|Delay 0.1)
        (Actor|Tick|SetActorTickEnabled true)
        (else
          (Actor|Tick|SetActorTickEnabled false))))))

(event Custom|关闭光剑
  (bind (_direction _新建轨迹_0) (Timeline|光剑动画 Reverse)
    (:Update
      (Transformation|SetRelativeScale3D (Variables|Default|GetScene1) (Math|Vector|MakeVector 1.0 1.0 _新建轨迹_0)))
    (:Finished
      (if (Utilities|Enum|Equal(Enum) _direction "Forward")
        (Variables|Default|Set上一帧位置 (Transformation|GetWorldLocation (Variables|Default|Get剑)))
        (Utilities|FlowControl|Delay 0.1)
        (Actor|Tick|SetActorTickEnabled true)
        (else
          (Actor|Tick|SetActorTickEnabled false))))))

(event EventTick
  (params (DeltaSeconds :type Float%20%28single-precision%29))
  (Variables|Default|Set挥剑速度 (/ (- (Transformation|GetWorldLocation (Variables|Default|Get剑)) (Variables|Default|Get上一帧位置)) DeltaSeconds))
  (CallFunction|伤害检测)
  (Variables|Default|Set上一帧位置 (Transformation|GetWorldLocation (Variables|Default|Get剑))))

(fn ConstructionScript)

(fn 计算挥剑末端速度
  (params (delta%20time :type Float%20%28double-precision%29))
  (Variables|Default|Set挥剑速度 (/ (- (Transformation|GetWorldLocation (Variables|Default|Get剑)) (Variables|Default|Get上一帧位置)) delta%20time))
  (Variables|Default|Set上一帧位置 (Transformation|GetWorldLocation (Variables|Default|Get剑))))

(fn 伤害检测
  (bind _剑 (Variables|Default|Get剑))
  (bind _returnvalue (Transformation|GetWorldLocation _剑))
  (bind (_outhit _returnvalue_2) (Collision|BoxTraceByChannel (Variables|Default|Get上一帧位置) _returnvalue (Math|Vector|MakeVector 1.0 1.0 5e+01) (Math|Rotator|MakeRotfromZX (Math|Vector|Normalize (- (Transformation|GetWorldLocation (Variables|Default|Get末端)) _returnvalue)) (Math|Vector|Normalize (Variables|Default|Get挥剑速度))) "TraceTypeQuery1" false 0 "None" true "(R=1.000000,G=0.000000,B=0.000000,A=1.000000)" "(R=0.000000,G=1.000000,B=0.000000,A=1.000000)" 3.0))
  (if _returnvalue_2
    (bind _asbp_方块 (Utilities|Casting|CastTobp_方块 (.HitActor (Collision|BreakHitResult _outhit))))
    (Class|伤害接口|施加伤害(Message) _asbp_方块 self (Utilities|Struct|Make剑hit (Variables|Default|Get挥剑速度) (Math|Vector|CrossProduct (Variables|Default|Get挥剑速度) (Math|Vector|GetForwardVector (Variables|Default|Get末端))) (.ImpactPoint (Collision|BreakHitResult _outhit)) _outhit))))

(fn 伤害目标)