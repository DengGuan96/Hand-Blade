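; Sword-reactive block (方块) that is either sliced apart or knocked away on the first damage event it receives.
; Construction copies its static mesh into a procedural mesh with convex collision and disables the original's collision.
; The damage event compares sword velocity relative to the block against a threshold.
; Fast hits slice along the swing plane with a capped cut and randomized impulses; slower hits enable physics and apply the relative velocity.
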(event Event施加伤害
  (params (触发者 :type Actor%20Object%20Reference) (NewParam :type 剑hit%20Structure))
  (bind _挥剑速度 (Utilities|Struct|Break剑hit NewParam))
  (bind _proceduralmesh (Variables|Default|GetProceduralMesh))
  (bind _returnvalue (Transformation|GetComponentVelocity _proceduralmesh))
  (bind _returnvalue_2 (- _挥剑速度 _returnvalue))
  (Utilities|FlowControl|DoOnce false
    (:Completed
      (if (>= (Math|Vector|VectorLength _returnvalue_2) 5.5e+02)
        (|切割效果 NewParam _returnvalue_2)
        (else
          (|打击效果 NewParam _returnvalue_2))))))

(fn ConstructionScript
  (bind _staticmesh (Variables|Default|GetStaticMesh))
  (Class|KismetProceduralMeshLibrary|CopyProceduralMeshfromStaticMeshComponent _staticmesh 0 (Variables|Default|GetProceduralMesh) true)
  (bind _vertices (Class|KismetProceduralMeshLibrary|GetSectionfromStaticMesh (Variables|/Script/Engine.StaticMeshComponent|GetStaticMesh _staticmesh)))
  (Class|ProceduralMeshComponent|AddCollisionConvexMesh (Variables|Default|GetProceduralMesh) _vertices)
  (Collision|SetCollisionEnabled (Variables|Default|GetStaticMesh) "NoCollision"))